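; Master RTS unit Blueprint with body and head meshes and decals that show selection state.
; The construction script applies meshes from MainStruct and the Color material.
; BeginPlay copies the player controller's unit color into Color and MainStruct, without reapplying it to the meshes.
; Tick lets the unit affect navigation generation only while stationary, disabling this as it moves.
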(event `self.ReceiveBeginPlay`
  (bind (_mainstruct_body _mainstruct_head _mainstruct_currenthp _mainstruct_maxhp) (break `/Game/Main/Blueprints/Libs/Structures/RTS_Units_MainStruct` (`self.MainStruct`)))
  (bind _asrts_player_controller_bp (cast `/Game/Main/Blueprints/Player/RTS_PlayerController_BP` (`GameplayStatics.GetPlayerController` 0)))
  (bind _output_get (set `self.PC` _asrts_player_controller_bp))
  (bind _output_get_2 (set `self.Color` (`/Game/Main/Blueprints/Player/RTS_PlayerController_BP.Color_Material_Unit` _output_get)))
  (set `self.MainStruct` (make `/Game/Main/Blueprints/Libs/Structures/RTS_Units_MainStruct` _mainstruct_body _mainstruct_head _mainstruct_currenthp _mainstruct_maxhp _output_get_2)))

(event `self.ReceiveTick`
  (params (DeltaSeconds :type "Float (single-precision)"))
  (if (> (`KismetMathLibrary.VSize` (`self.GetVelocity`)) 0.0)
    (`self.SetCanAffectNavigationGeneration` false)
    (else
      (`self.SetCanAffectNavigationGeneration` true))))

(fn `SetDeselectedDecal`
  (`SceneComponent.SetVisibility` (`self.DeselectedDecal`) true false)
  (`SceneComponent.SetVisibility` (`self.SelectedDecal`) false false))

(fn `SetSelectedDecal`
  (`SceneComponent.SetVisibility` (`self.DeselectedDecal`) false false)
  (`SceneComponent.SetVisibility` (`self.SelectedDecal`) true false))

(fn `UserConstructionScript`
  (bind (_mainstruct_body _mainstruct_head) (break `/Game/Main/Blueprints/Libs/Structures/RTS_Units_MainStruct` (`self.MainStruct`)))
  (`SkinnedMeshComponent.SetSkinnedAssetAndUpdate` (`self.Mesh`) _mainstruct_body false)
  (`SkinnedMeshComponent.SetSkinnedAssetAndUpdate` (`self.Head`) _mainstruct_head false)
  (`PrimitiveComponent.SetMaterial` (`self.Mesh`) 0 (`self.Color`))
  (`PrimitiveComponent.SetMaterial` (`self.Head`) 0 (`self.Color`)))