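; UnitMaster_BP is a unit Blueprint, named as a master for units, that shows whether the unit is selected through two decal components.
; SetSelectedDecal shows SelectedDecal and hides DeselectedDecal, and SetDeselectedDecal does the reverse, each toggling both visibility and hidden-in-game.
; BeginPlay, Tick and the construction script are empty, so the switch happens only when these functions are called.
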(event `self.ReceiveBeginPlay`)

(event `self.ReceiveTick`
  (params (DeltaSeconds :type "Float (single-precision)")))

(fn `SetDeselectedDecal`
  (bind _deselecteddecal (`self.DeselectedDecal`))
  (bind _selecteddecal (`self.SelectedDecal`))
  (`SceneComponent.SetVisibility` _deselecteddecal true false)
  (`SceneComponent.SetHiddenInGame` _deselecteddecal false false)
  (`SceneComponent.SetVisibility` _selecteddecal false false)
  (`SceneComponent.SetHiddenInGame` _selecteddecal true false))

(fn `SetSelectedDecal`
  (bind _deselecteddecal (`self.DeselectedDecal`))
  (bind _selecteddecal (`self.SelectedDecal`))
  (`SceneComponent.SetVisibility` _deselecteddecal false false)
  (`SceneComponent.SetHiddenInGame` _deselecteddecal true false)
  (`SceneComponent.SetVisibility` _selecteddecal true false)
  (`SceneComponent.SetHiddenInGame` _selecteddecal false false))

(fn `UserConstructionScript`)