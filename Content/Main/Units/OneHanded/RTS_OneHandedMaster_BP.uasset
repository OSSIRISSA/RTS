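; RTS_OneHandedMaster_BP is the master Blueprint for one-handed RTS units that carry a weapon and shield.
; Its construction script calls the parent's, then assigns the Weapon mesh to WeaponR and the Shield mesh to WeaponL.
; It also sets the one-handed anim Blueprint on the body mesh and applies the Color material to slot 0 of both held meshes.
; The event graph contains only disabled or empty placeholder events.
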(fn `UserConstructionScript`
  (`parent.UserConstructionScript`)
  (`StaticMeshComponent.SetStaticMesh` (`self.Weapon_R`) (`self.Weapon`))
  (`StaticMeshComponent.SetStaticMesh` (`self.Weapon_L`) (`self.Shield`))
  (`SkeletalMeshComponent.SetAnimInstanceClass` (`self.Mesh`) "/Game/Main/Units/OneHanded/RTS_OneHandedAnimBP.RTS_OneHandedAnimBP_C")
  (`PrimitiveComponent.SetMaterial` (`self.Weapon_R`) 0 (`self.Color`))
  (`PrimitiveComponent.SetMaterial` (`self.Weapon_L`) 0 (`self.Color`)))