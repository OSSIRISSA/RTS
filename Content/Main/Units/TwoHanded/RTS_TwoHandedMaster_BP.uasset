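; Master Blueprint for two-handed weapon units in the RTS, extending a parent unit class.
; Its construction script runs the parent's, then sets the right-hand weapon mesh from the two-handed struct and assigns the two-handed Animation Blueprint to the mesh.
; It also applies the main struct's color material to the weapon.
; BeginPlay and Tick only call the parent.
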(event `self.ReceiveBeginPlay`
  (`parent.ReceiveBeginPlay`))

(event `self.ReceiveTick`
  (params (DeltaSeconds :type "Float (single-precision)"))
  (`parent.ReceiveTick` DeltaSeconds))

(fn `UserConstructionScript`
  (bind _twohandedmainstruct_weapon_r (break `/Game/Main/Blueprints/Libs/Structures/RTS_TwoHandedUnits_Struct` (`self.TwoHandedMainStruct`)))
  (bind (_mainstruct_body _mainstruct_head _mainstruct_currenthp _mainstruct_maxhp _mainstruct_color) (break `/Game/Main/Blueprints/Libs/Structures/RTS_Units_MainStruct` (`self.MainStruct`)))
  (`parent.UserConstructionScript`)
  (`StaticMeshComponent.SetStaticMesh` (`self.Weapon_R`) _twohandedmainstruct_weapon_r)
  (`SkeletalMeshComponent.SetAnimInstanceClass` (`self.Mesh`) "/Game/Main/Units/TwoHanded/RTS_TwoHandedAnimBP.RTS_TwoHandedAnimBP_C")
  (`PrimitiveComponent.SetMaterial` (`self.Weapon_R`) 0 _mainstruct_color))