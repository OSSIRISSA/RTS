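; RTS_Builder_BP is the two-handed builder unit Blueprint for an RTS.
; It offers three functions that swap the static mesh on the WeaponR component to a pickaxe, axe or hammer.
; The construction script only calls its parent, and nothing in this Blueprint decides when the tool changes.
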(fn `SetAxe`
  (`StaticMeshComponent.SetStaticMesh` (`self.Weapon_R`) (`self.Axe`)))

(fn `SetHammer`
  (`StaticMeshComponent.SetStaticMesh` (`self.Weapon_R`) (`self.Hammer`)))

(fn `SetPickaxe`
  (`StaticMeshComponent.SetStaticMesh` (`self.Weapon_R`) (`self.Pickaxe`)))

(fn `UserConstructionScript`
  (`parent.UserConstructionScript`))