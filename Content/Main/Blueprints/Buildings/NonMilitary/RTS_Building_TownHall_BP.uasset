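; Town Hall building for the RTS, extending a parent building class with a selection UI and timed tasks.
; Selection lazily creates or re-adds the TownHall widget, setting action panel visibility from readiness and player color match; deselection or death removes it.
; A single timeline, rate-scaled to each task's duration, feeds progress and completion to the widget.
; Capsule end-overlap completes the last task again when production is ready.
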(event `self.Ready`
  (`parent.Ready`)
  (`Widget.SetVisibility` (`/Game/Main/Blueprints/Widgets/Buildings/TownHall/RTS_TownHall_ControllPannel_WBP.Main_Surface` (`self.WidgetRef`)) "Visible")
  (`Widget.SetVisibility` (`/Game/Main/Blueprints/Widgets/Buildings/TownHall/RTS_TownHall_ControllPannel_WBP.BaseActions` (`self.WidgetRef`)) "Visible"))

(event `self.Event_SetDeselected`
  (`parent.Event_SetDeselected`)
  (bind _widgetref (`self.WidgetRef`)
    (:`then`
      (`Widget.RemoveFromParent` _widgetref))
    (:`else`)))

(event `self.Event_SetSelected`
  (bind _playercontrollerref (`self.PlayerControllerRef`))
  (`parent.Event_SetSelected`)
  (bind _widgetref (`self.WidgetRef`)
    (:`then`
      (`UserWidget.AddToViewport` _widgetref 0))
    (:`else`
      (bind _returnvalue (`|CreateWidget` (`self.TownHall_WBP`) _playercontrollerref _playercontrollerref self))
      (bind _output_get (set `self.WidgetRef` _returnvalue))
      (`UserWidget.AddToViewport` _output_get 0)))
  (`Widget.SetVisibility` (`/Game/Main/Blueprints/Widgets/Buildings/TownHall/RTS_TownHall_ControllPannel_WBP.Main_Surface` (`self.WidgetRef`)) (select `bool` (`self.IsReady?`) :`false` "Hidden" :`true` "Visible" :!type "ESlateVisibility Enum"))
  (`Widget.SetVisibility` (`/Game/Main/Blueprints/Widgets/Buildings/TownHall/RTS_TownHall_ControllPannel_WBP.BaseActions` (`self.WidgetRef`)) (select `bool` (`self.IsReady?`) :`false` "Hidden" :`true` "Visible" :!type "ESlateVisibility Enum"))
  (`Widget.SetVisibility` (`/Game/Main/Blueprints/Widgets/Buildings/TownHall/RTS_TownHall_ControllPannel_WBP.Main_Surface` (`self.WidgetRef`)) (select `bool` (== (`/Game/Main/Blueprints/Player/RTS_PlayerController_BP.Color_Material_Building` (`/Game/Main/Blueprints/Buildings/RTS_BuildingMaster_BP.PlayerControllerRef` (`/Game/Main/Blueprints/Widgets/Buildings/TownHall/RTS_TownHall_ControllPannel_WBP.Building` (`self.WidgetRef`)))) (`/Game/Main/Blueprints/Buildings/RTS_BuildingMaster_BP.Color` (`/Game/Main/Blueprints/Widgets/Buildings/TownHall/RTS_TownHall_ControllPannel_WBP.Building` (`self.WidgetRef`)))) :`false` "Hidden" :`true` "Visible" :!type "ESlateVisibility Enum"))
  (`Widget.SetVisibility` (`/Game/Main/Blueprints/Widgets/Buildings/TownHall/RTS_TownHall_ControllPannel_WBP.BaseActions` (`self.WidgetRef`)) (select `bool` (== (`/Game/Main/Blueprints/Player/RTS_PlayerController_BP.Color_Material_Building` (`/Game/Main/Blueprints/Buildings/RTS_BuildingMaster_BP.PlayerControllerRef` (`/Game/Main/Blueprints/Widgets/Buildings/TownHall/RTS_TownHall_ControllPannel_WBP.Building` (`self.WidgetRef`)))) (`/Game/Main/Blueprints/Buildings/RTS_BuildingMaster_BP.Color` (`/Game/Main/Blueprints/Widgets/Buildings/TownHall/RTS_TownHall_ControllPannel_WBP.Building` (`self.WidgetRef`)))) :`false` "Hidden" :`true` "Visible" :!type "ESlateVisibility Enum")))

(event `Stop_Task`
  (bind (_direction _percentage) (`Timeline|Task` :!via `Stop` :!label _label)
    (:`Update`
      (`/Game/Main/Blueprints/Widgets/Buildings/TownHall/RTS_TownHall_ControllPannel_WBP.Update_Percent` (`self.WidgetRef`) _percentage))
    (:`Finished`
      (`/Game/Main/Blueprints/Widgets/Buildings/TownHall/RTS_TownHall_ControllPannel_WBP.Task_Finished` (`self.WidgetRef`) (`self.LastTask`)))))

(event `Start_Task`
  (params (Task :type "Widget Object Reference") (Time :type "Float (double-precision)"))
  (set `self.LastTask` Task)
  (`TimelineComponent.SetPlayRate` (`self.Task`) (/ 1.0 Time))
  (goto _label :!via `PlayFromStart`))

(event `self.Death`
  (`parent.Death`)
  (`Widget.RemoveFromParent` (`self.WidgetRef`)))

(event `self.CheckCapsuleEndOverlap`
  (bind _widgetref (`self.WidgetRef`)
    (:`then`
      (if (`/Game/Main/Blueprints/Widgets/Buildings/TownHall/RTS_TownHall_ControllPannel_WBP.IsProductionReady?` _widgetref)
        (bind _lasttask (`self.LastTask`)
          (:`then`
            (`/Game/Main/Blueprints/Widgets/Buildings/TownHall/RTS_TownHall_ControllPannel_WBP.Task_Finished` (`self.WidgetRef`) _lasttask))
          (:`else`))))
    (:`else`)))

(event `self.UpdateHP`
  (bind _widgetref (`self.WidgetRef`)
    (:`then`
      (`/Game/Main/Blueprints/Widgets/Buildings/TownHall/RTS_TownHall_ControllPannel_WBP.UpdateHP` _widgetref))
    (:`else`)))

(fn `UserConstructionScript`
  (`parent.UserConstructionScript`))