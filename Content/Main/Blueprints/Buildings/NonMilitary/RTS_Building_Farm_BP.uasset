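; Farm building Blueprint for the RTS, a non-military building that extends a parent building class and manages an on-screen panel while selected.
; Selection shows a cached widget, created on first use from TownHallWBP with the player controller and building passed in.
; Deselection and death remove the widget, and HP updates are forwarded to it.
; Death removes it without the validity check used elsewhere.
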(event `self.Event_SetSelected`
  (bind _playercontrollerref (`self.PlayerControllerRef`))
  (`parent.Event_SetSelected`)
  (bind _widgetref (`self.WidgetRef`)
    (:`then`
      (`UserWidget.AddToViewport` _widgetref 0))
    (:`else`
      (bind _returnvalue (`|CreateWidget` (`self.TownHall_WBP`) _playercontrollerref _playercontrollerref self))
      (bind _output_get (set `self.WidgetRef` _returnvalue))
      (`UserWidget.AddToViewport` _output_get 0))))

(event `self.Event_SetDeselected`
  (`parent.Event_SetDeselected`)
  (bind _widgetref (`self.WidgetRef`)
    (:`then`
      (`Widget.RemoveFromParent` _widgetref))
    (:`else`)))

(event `self.Death`
  (`parent.Death`)
  (`Widget.RemoveFromParent` (`self.WidgetRef`)))

(event `self.UpdateHP`
  (bind _widgetref (`self.WidgetRef`)
    (:`then`
      (`/Game/Main/Blueprints/Widgets/Buildings/Farm/RTS_Farm_ControllPannel_WBP.UpdateHP` _widgetref))
    (:`else`)))

(fn `UserConstructionScript`
  (`parent.UserConstructionScript`))