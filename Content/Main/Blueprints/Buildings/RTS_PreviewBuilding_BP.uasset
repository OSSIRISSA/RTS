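; RTS building placement preview actor that shows a ghost mesh at the cursor while building mode is active on the player controller.
; ConstructBuilding briefly spawns the requested building class to read its display mesh, starts the preview, then destroys that temporary actor.
; While the gate is open, Tick moves the preview to the supplied cursor position with a fixed XY offset and swaps to a bad-placement material when any actor overlaps.
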(event `DestroyPreview`
  (`self.CloseGate`)
  (set `self.Building Class` null)
  (set `self.Display Mesh` null)
  (bind _output_get (set `self.IsPreviewing?` false))
  (`/Game/Main/Blueprints/Player/RTS_PlayerController_BP.SetBuildingModeActive` (`self.PlayerControllerRef`) _output_get)
  (`StaticMeshComponent.SetStaticMesh` (`self.PreviewBuilding`) (`self.Display Mesh`)))

(event `/Game/Main/Blueprints/Libraries/RTS_Construction_IF.ConstructBuilding`
  (params (BuildingMasterClass :type "/Game/Main/Blueprints/Buildings/RTS_BuildingMaster_BP Class Reference"))
  (bind _returnvalue (`|SpawnActorFromClass` BuildingMasterClass (`KismetMathLibrary.MakeTransform` (0.0 0.0 0.0)) "AlwaysSpawn" "OverrideRootScale" null (`self.PlayerControllerRef`) null))
  (`|ExecutionSequence`
    (:`then_0`
      (bind _asrts_building_master_bp (castclass `/Game/Main/Blueprints/Buildings/RTS_BuildingMaster_BP` BuildingMasterClass))
      (`self.DestroyPreview`)
      (`self.SpawnPreview` _asrts_building_master_bp (`/Game/Main/Blueprints/Buildings/RTS_BuildingMaster_BP.DisplayMesh` _returnvalue)))
    (:`then_1`
      (`self.K2_DestroyActor` _returnvalue))))

(event `SpawnPreview`
  (params (BuildingClass :type "/Game/Main/Blueprints/Buildings/RTS_BuildingMaster_BP Class Reference") (DisplayMesh :type "StaticMesh Object Reference"))
  (if (`self.IsPreviewing?`)
    (`self.DestroyPreview`))
  (set `self.Building Class` BuildingClass)
  (set `self.Display Mesh` DisplayMesh)
  (bind _output_get (set `self.IsPreviewing?` true))
  (`/Game/Main/Blueprints/Player/RTS_PlayerController_BP.SetBuildingModeActive` (`self.PlayerControllerRef`) _output_get)
  (`StaticMeshComponent.SetStaticMesh` (`self.PreviewBuilding`) (`self.Display Mesh`))
  (`self.OpenGate`))

(event `self.ReceiveTick`
  (params (DeltaSeconds :type "Float (single-precision)"))
  (bind _previewbuilding (`self.PreviewBuilding`))
  (`/Engine/EditorBlueprintResources/StandardMacros.Gate` true :!label _label
    (:`Exit`
      (`self.K2_SetActorLocation` self (`self.GridSnaps`) true true)
      (if (`self.CheckOverlap`)
        (`PrimitiveComponent.SetMaterial` _previewbuilding 0 "/Game/Main/Assets/Materials/Preview/PreviewBad_Mat_Inst.PreviewBad_Mat_Inst")
        (else
          (`PrimitiveComponent.SetMaterial` _previewbuilding 0 "/Game/Main/Assets/Materials/Preview/Preview_Mat_Inst.Preview_Mat_Inst"))))))

(event `OpenGate`
  (goto _label :!via `Open`))

(event `CloseGate`
  (goto _label :!via `Close`))

(fn `CheckOverlap`
  (returns (IsOverlapping :type Boolean))
  (return (>= (`KismetArrayLibrary.Array_LastIndex` (`self.GetOverlappingActors` null)) 0)))

(fn `GetCursorPosition`
  (params (`Cursor Location In` :type "Vector Structure"))
  (set `self.CursorWorldPosition` `Cursor Location In`)
  (return))

(fn `GridSnaps`
  (returns (Output :type "Vector Structure"))
  (bind (_cursorworldposition_x _cursorworldposition_y _cursorworldposition_z) (`KismetMathLibrary.BreakVector` (`self.CursorWorldPosition`)))
  (return (`KismetMathLibrary.MakeVector` (+ _cursorworldposition_x 50.0) (+ _cursorworldposition_y 50.0) _cursorworldposition_z)))

(fn `UserConstructionScript`)