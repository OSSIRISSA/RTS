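; Farm building Blueprint for the RTS residential set, a thin child that defers its behavior to a parent class.
; BeginPlay branches on Placed, running Collisions when set and the parent BeginPlay otherwise.
; Tick reaches the parent through a Gate fed by Placed.
; The construction script and Collisions override only call their parent versions.
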(event `self.ReceiveBeginPlay`
  (if (`self.Placed`)
    (`self.Collisions`)
    (else
      (`parent.ReceiveBeginPlay`))))

(event `self.ReceiveTick`
  (params (DeltaSeconds :type "Float (single-precision)"))
  (`/Engine/EditorBlueprintResources/StandardMacros.Gate` (`self.Placed`)
    (:`Exit`
      (`parent.ReceiveTick` DeltaSeconds))))

(fn `Collisions`
  (`parent.Collisions`))

(fn `UserConstructionScript`
  (`parent.UserConstructionScript`))