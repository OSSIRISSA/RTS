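; Master RTS building actor that covers cursor-following placement preview and timed construction.
; On Tick, a gate moves it to the cursor and swaps good/bad preview materials by box overlap until Place closes it and zeroes HP.
; Building opens a second gate that interpolates HP toward max, updates the HUD and swaps staged meshes by HP ratio.
; Colide makes the mesh blocking, except on Visibility, and destroys the overlap box.
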(event `self.ReceiveBeginPlay`
  ;[1 0 0] BP
  (bind _asrts_player_controller_bp (cast `/Game/Main/Blueprints/Player/RTS_PlayerController_BP` (`GameplayStatics.GetPlayerController` 0)))
  (bind _output_get (set `self.PlayerControllerRef` _asrts_player_controller_bp))
  (set `/Game/Main/Blueprints/Player/RTS_PlayerController_BP.Preview_Ref` self _output_get)
  (set `self.Color` (`/Game/Main/Blueprints/Player/RTS_PlayerController_BP.Color_Material_Building` _output_get))
  (set `self.Start` true))

(event `Colide`
  (`self.Collisions`))

(event `self.ReceiveTick`
  (params (DeltaSeconds :type "Float (single-precision)"))
  (bind (_main_struct_building0 _main_struct_building50 _main_struct_building100 _main_struct_name _main_struct_current_hp _main_struct_max_hp) (break `/Game/Main/Blueprints/Structures/RTS_Building_Struct` (`self.Main_Struct`)))
  (bind (_main_struct_building0_2 _main_struct_building50_2 _main_struct_building100_2) (break `/Game/Main/Blueprints/Structures/RTS_Building_Struct` (`self.Main_Struct`)))
  (bind (_main_struct_building0_3 _main_struct_building50_3 _main_struct_building100_3 _main_struct_name_2 _main_struct_current_hp_2 _main_struct_max_hp_2) (break `/Game/Main/Blueprints/Structures/RTS_Building_Struct` (`self.Main_Struct`)))
  (bind _main_struct_building0_4 (break `/Game/Main/Blueprints/Structures/RTS_Building_Struct` (`self.Main_Struct`)))
  (bind (_main_struct_building0_5 _main_struct_building50_4) (break `/Game/Main/Blueprints/Structures/RTS_Building_Struct` (`self.Main_Struct`)))
  (bind _returnvalue (/ (`KismetMathLibrary.Conv_IntToDouble` _main_struct_current_hp) (`KismetMathLibrary.Conv_IntToDouble` _main_struct_max_hp)))
  (if (`self.Start`)
    (`|ExecutionSequence`
      (:`then_0`
        (`/Engine/EditorBlueprintResources/StandardMacros.Gate` false :!label _label
          (:`Exit`
            (`|ExecutionSequence`
              (:`then_0`
                (`self.SetMouseCursorLocation`))
              (:`then_1`
                (`self.MoveBuildingToCursor`))))))
      (:`then_1`
        (`/Engine/EditorBlueprintResources/StandardMacros.Gate` true :!label _label_2
          (:`Exit`
            (set `self.Main_Struct` (make `/Game/Main/Blueprints/Structures/RTS_Building_Struct` _main_struct_building0 _main_struct_building50 _main_struct_building100 _main_struct_name (`KismetMathLibrary.FTrunc` (`KismetMathLibrary.FInterpTo_Constant` (`KismetMathLibrary.Conv_IntToDouble` _main_struct_current_hp_2) (`KismetMathLibrary.Conv_IntToDouble` _main_struct_max_hp_2) (`/Game/Main/Blueprints/Player/RTS_PlayerController_BP.Delta` (`self.PlayerControllerRef`)) 100.0)) _main_struct_max_hp))
            (`/Game/Main/Blueprints/Widgets/Main_WBP.UpdatePB/HP/Percent` (`/Game/Main/Blueprints/Player/RTS_PlayerController_BP.Main_HUD` (`self.PlayerControllerRef`)) self)
            (if (`KismetMathLibrary.InRange_FloatFloat` _returnvalue 0.0 0.5 true false)
              (`/Engine/EditorBlueprintResources/StandardMacros.DoOnce` false
                (:`Completed`
                  (`StaticMeshComponent.SetStaticMesh` (`self.BuildingMesh`) _main_struct_building0_4)))
              (elif (`KismetMathLibrary.InRange_FloatFloat` _returnvalue 0.5 1.0 true false)
                (`/Engine/EditorBlueprintResources/StandardMacros.DoOnce` false
                  (:`Completed`
                    (`StaticMeshComponent.SetStaticMesh` (`self.BuildingMesh`) _main_struct_building50_4)))
                (else
                  (`/Engine/EditorBlueprintResources/StandardMacros.DoOnce` false
                    (:`Completed`
                      (`StaticMeshComponent.SetStaticMesh` (`self.BuildingMesh`) _main_struct_building100_2))))))))))))

(event `Place`
  (bind (_main_struct_building0 _main_struct_building50 _main_struct_building100 _main_struct_name _main_struct_current_hp _main_struct_max_hp) (break `/Game/Main/Blueprints/Structures/RTS_Building_Struct` (`self.Main_Struct`)))
  (set `self.Main_Struct` (make `/Game/Main/Blueprints/Structures/RTS_Building_Struct` _main_struct_building0 _main_struct_building50 _main_struct_building100 _main_struct_name 0 _main_struct_max_hp))
  (goto _label :!via `Close`))

(event `Building`
  (bind (_main_struct_building0 _main_struct_building50 _main_struct_building100 _main_struct_name _main_struct_current_hp _main_struct_max_hp) (break `/Game/Main/Blueprints/Structures/RTS_Building_Struct` (`self.Main_Struct`)))
  (`StaticMeshComponent.SetStaticMesh` (`self.BuildingMesh`) _main_struct_building0)
  (`PrimitiveComponent.SetMaterial` (`self.BuildingMesh`) 0 (`self.Color`))
  (goto _label_2 :!via `Open`))

(fn `CheckOverlap`
  (returns (IsOverlapping :type Boolean))
  (return (>= (`KismetArrayLibrary.Array_LastIndex` (`PrimitiveComponent.GetOverlappingActors` (`self.Box`) null)) 0)))

(fn `Collisions`
  (`PrimitiveComponent.SetCollisionResponseToAllChannels` (`self.BuildingMesh`) "ECR_Block")
  (`ActorComponent.K2_DestroyComponent` (`self.Box`))
  (`PrimitiveComponent.SetCollisionResponseToChannel` (`self.BuildingMesh`) "ECC_Visibility" "ECR_Ignore"))

(fn `GridSnaps`
  (returns (Output :type "Vector Structure"))
  (locals (AddValueX :type "Float (double-precision)") (AddValueY :type "Float (double-precision)" :default 0.0))
  (bind (_cursorposition_x _cursorposition_y _cursorposition_z) (`KismetMathLibrary.BreakVector` (`self.CursorPosition`)))
  (return (`KismetMathLibrary.MakeVector` (+ _cursorposition_x (`local.AddValueX`)) (+ _cursorposition_y (`local.AddValueY`)) _cursorposition_z)))

(fn `UserConstructionScript`
  (`StaticMeshComponent.SetStaticMesh` (`self.BuildingMesh`) (`.Building100_24_72E1676540B065CCABD33B87FD547AB4` (break `/Game/Main/Blueprints/Structures/RTS_Building_Struct` (`self.Main_Struct`))))
  (`PrimitiveComponent.SetMaterial` (`self.BuildingMesh`) 0 (`self.Color`)))