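; Barracks building Blueprint for the RTS military buildings, deferring its placement and collision logic to a parent class.
; BeginPlay calls Collisions when the building is already Placed, otherwise it runs the parent's BeginPlay.
; A Gate, starting closed if Placed, passes Tick to the parent until Place runs the parent logic and closes it, stopping parent ticking for placed buildings.
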(event `self.ReceiveBeginPlay`
  (if (`self.Placed`)
    (`self.Collisions`)
    (else
      (`parent.ReceiveBeginPlay`))))

(event `self.ReceiveTick`
  (params (DeltaSeconds :type "Float (single-precision)"))
  (`/Engine/EditorBlueprintResources/StandardMacros.Gate` (`self.Placed`) :!label _label
    (:`Exit`
      (`parent.ReceiveTick` DeltaSeconds))))

(event `self.Place`
  (`parent.Place`)
  (goto _label :!via `Close`))

(fn `Collisions`
  (`parent.Collisions`))

(fn `UserConstructionScript`
  (`parent.UserConstructionScript`))