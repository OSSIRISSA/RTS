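; Blueprint function library of RTS helpers for cursor tracing, actor facing and filtered line traces.
; SetCursorWorldPosition deprojects the mouse and returns the Visibility trace's hit location when the hit-actor check passes.
; RotateActorToTheRotator applies the look-at yaw from one actor toward another, named Rotator.
; GetWayToTheItem returns a trace's hit location, ignoring every actor of a given class except the specified one.
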(fn `GetWayToTheItem`
  (params (TraceChannel :type "ETraceTypeQuery Enum" :default "TraceTypeQuery1") (Start :type "Vector Structure") (End :type "Vector Structure") (ActorNotToIgnore :type "Actor Object Reference (by ref)") (ClassToIgnore :type "Actor Class Reference"))
  (returns (Location :type "Vector Structure"))
  (bind _outactors (`GameplayStatics.GetAllActorsOfClass` null ClassToIgnore))
  (`KismetArrayLibrary.Array_RemoveItem` _outactors ActorNotToIgnore)
  (bind _outhit (`KismetSystemLibrary.LineTraceSingle` null Start End TraceChannel false _outactors))
  (return (`.Location` (`GameplayStatics.BreakHitResult` _outhit))))

(fn `RotateActorToTheRotator`
  (params (Actor :type "Actor Object Reference") (Rotator :type "Actor Object Reference"))
  (bind (_returnvalue_roll _returnvalue_pitch _returnvalue_yaw) (`KismetMathLibrary.BreakRotator` (`KismetMathLibrary.FindLookAtRotation` (`Actor.K2_GetActorLocation` Actor) (`Actor.K2_GetActorLocation` Rotator))))
  (`/Engine/EditorBlueprintResources/StandardMacros.IsValid` Actor
    (:`Is Valid`
      (`Actor.K2_SetActorRotation` Actor (`KismetMathLibrary.MakeRotator` 0.0 0.0 _returnvalue_yaw) false))))

(fn `SetCursorWorldPosition`
  (params (Controller :type "/Game/Main/Blueprints/Player/RTS_PlayerController_BP Object Reference") (SightDistance :type "Float (double-precision)"))
  (returns (RelativeCoursorLocationInGame :type "Vector Structure"))
  (bind (_worldlocation _worlddirection) (`PlayerController.DeprojectMousePositionToWorld` Controller))
  (bind _outhit (`KismetSystemLibrary.LineTraceSingle` null _worldlocation (+ _worldlocation (* _worlddirection SightDistance)) "TraceTypeQuery1"))
  (if (!= (`.HitActor` (`GameplayStatics.BreakHitResult` _outhit)) null)
    (return (`.Location` (`GameplayStatics.BreakHitResult` _outhit)))))