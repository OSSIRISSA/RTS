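; ResourceMaster_BP is, going by its name, the base actor for resources, and it varies the look of each instance's ResourceMesh.
; Its Construction Script optionally gives the mesh a random world scale between MinMeshSize and MaxMeshSize, rolled separately per axis so proportions vary.
; A second flag optionally sets a random yaw, with pitch and roll at zero.
; The event graph holds only disabled placeholder events, with no runtime logic.
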(fn `UserConstructionScript`
  (bind _returnvalue (`KismetMathLibrary.RandomFloatInRange` (`self.MinMeshSize`) (`self.MaxMeshSize`)))
  (if (`self.IsRandomSize`)
    (`SceneComponent.SetWorldScale3D` (`self.ResourceMesh`) (`KismetMathLibrary.MakeVector` _returnvalue _returnvalue _returnvalue)))
  (if (`self.IsRandomRotation`)
    (`SceneComponent.K2_SetWorldRotation` (`self.ResourceMesh`) (`KismetMathLibrary.MakeRotator` 0.0 0.0 (`KismetMathLibrary.RandomFloatInRange` 0.0 360.0)) false false)))