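; RTS resource spawner actor that scatters resource actors at random points inside its SpawnVolume box.
; On BeginPlay, if IsSpawnedOnBP is set, it picks one random class from ResourceRef and passes it to SpawnResource with SpawnAmount.
; SpawnResource takes a class and count, then spawns that many copies, each at a new random point within the volume's scaled extent.
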(event `self.ReceiveBeginPlay`
  (if (`self.IsSpawnedOnBP`)
    (`self.SpawnResource` (`KismetArrayLibrary.Array_Random` (`self.ResourceRef`)) (`self.SpawnAmount`))))

(fn `SpawnResource`
  (params (Resource :type "/Game/Main/Blueprints/Resources/RTS_ResourceMaster_BP Class Reference") (SpawnAmount :type Integer))
  (locals (Resource_Ref_L :type "/Game/Main/Blueprints/Resources/RTS_ResourceMaster_BP Class Reference") (SpawnAmount_L :type Integer))
  (bind _spawnvolume (`self.SpawnVolume`))
  (set `local.Resource_Ref_L` Resource)
  (set `local.SpawnAmount_L` SpawnAmount)
  (for _ (range 1 (+ (`self.SpawnAmount`) 1))
    (`|SpawnActorFromClass` (`local.Resource_Ref_L`) (`KismetMathLibrary.MakeTransform` (`KismetMathLibrary.RandomPointInBoundingBox` (`SceneComponent.K2_GetComponentLocation` _spawnvolume) (`BoxComponent.GetScaledBoxExtent` _spawnvolume))) "Undefined" "OverrideRootScale" null null)))

(fn `UserConstructionScript`)