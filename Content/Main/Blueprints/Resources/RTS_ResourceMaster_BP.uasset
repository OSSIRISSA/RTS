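; Base RTS resource actor that holds a harvestable amount and can be shown as selected.
; Harvesting arrives as damage that subtracts from the amount; on depletion it stores the remainder as the per-collection yield and hides the actor rather than destroying it.
; The construction script optionally randomizes the mesh's per-axis scale and yaw for variety.
; Select and deselect functions toggle the Selection component's visibility.
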(event `self.ReceiveAnyDamage`
  (params (Damage :type "Float (single-precision)") (DamageType :type "DamageType Object Reference") (InstigatedBy :type "Controller Object Reference") (DamageCauser :type "Actor Object Reference"))
  (if (>= Damage (`KismetMathLibrary.Conv_IntToDouble` (`self.ResourceAmount`)))
    (set `self.CollectPerTime` (`self.ResourceAmount`))
    (set `self.ResourceAmount` 0)
    (`self.SetActorHiddenInGame` true)
    (else
      (set `self.ResourceAmount` (- (`self.ResourceAmount`) (`KismetMathLibrary.FTrunc` Damage))))))

(event `self.ReceiveTick`
  (params (DeltaSeconds :type "Float (single-precision)")))

(fn `SetDeselected`
  (`SceneComponent.SetVisibility` (`self.Selection`) false false))

(fn `SetSelected`
  (`SceneComponent.SetVisibility` (`self.Selection`) true false))

(fn `UserConstructionScript`
  (bind _returnvalue (`KismetMathLibrary.RandomFloatInRange` (`self.MinMeshSize`) (`self.MaxMeshSize`)))
  (if (`self.IsRandomSize`)
    (`SceneComponent.SetWorldScale3D` (`self.ResourceMesh`) (`KismetMathLibrary.MakeVector` _returnvalue _returnvalue _returnvalue)))
  (if (`self.IsRandomRotation`)
    (`SceneComponent.K2_SetWorldRotation` (`self.ResourceMesh`) (`KismetMathLibrary.MakeRotator` 0.0 0.0 (`KismetMathLibrary.RandomFloatInRange` 0.0 360.0)) false false)))