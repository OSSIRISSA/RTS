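; RTS player controller that drives the camera pawn, unit and building selection, unit orders and building placement, and creates the main HUD.
; Input pans, rotates, zooms and edge-scrolls the camera; hold-to-select goes through the marquee HUD, and cursor traces select buildings.
; Right-click cancels placement or sends selected units via AI MoveTo with a decal; left-click places previews and dispatches the nearest non-busy unit.
; It also picks team color materials and has a temporary debug unit-spawn key.
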(event `self.ReceiveBeginPlay`
  ;[1 0 0] BeginPlay
  (`|ExecutionSequence`
    (:`then_0`
      (`self.ReferenceCast`))
    (:`then_1`
      (`self.SpawnWidgets`)
      (`UserWidget.AddToViewport` (`self.Main_HUD`) 0)
      (`self.SetHUDVisibility` "Visible"))
    (:`then_2`
      (`WidgetBlueprintLibrary.SetInputMode_GameAndUIEx` self null "DoNotLock" false))
    (:`then_3`
      (`self.SetColor`))))

(event `InputAction|ZoomIn`
  (params (Key :type "Key Structure"))
  (bind _springarm (`/Game/Main/Blueprints/Player/RTS_CameraPawn_BP.SpringArm` (`self.Camera_Pawn_Ref`)))
  ;[0 1 1] Movement
  ;;[1 1 1] Zoom In
  (:`Pressed`
    (if (`self.Zoom?`)
      (set `SpringArmComponent.TargetArmLength` (`KismetMathLibrary.FClamp` (- (`SpringArmComponent.TargetArmLength` _springarm) (`self.ZoomSpeed`)) (`self.MinZoomLim`) (`self.MaxZoomLim`)) _springarm))))

(event `InputAction|Rotate`
  (params (Key :type "Key Structure"))
  (bind _camera_pawn_ref (`self.Camera_Pawn_Ref`))
  (bind (_returnvalue_roll _returnvalue_pitch _returnvalue_yaw) (`KismetMathLibrary.BreakRotator` (`self.K2_GetActorRotation` _camera_pawn_ref)))
  ;[0 1 1] Movement
  ;;[1 1 1] Rotate X
  (:`Pressed`
    (if (`self.Rotate?`)
      (goto _label :!via `Open`)))
  (:`Released`
    (goto _label :!via `Close`)))

(event `InputAxisKey|MouseX`
  (params (AxisValue :type "Float (single-precision)"))
  (bind _camera_pawn_ref (`self.Camera_Pawn_Ref`))
  (bind (_returnvalue_roll _returnvalue_pitch _returnvalue_yaw) (`KismetMathLibrary.BreakRotator` (`self.K2_GetActorRotation` _camera_pawn_ref)))
  ;[0 1 1] Movement
  ;;[1 1 1] Rotate X
  (`/Engine/EditorBlueprintResources/StandardMacros.Gate` true :!label _label
    (:`Exit`
      (`self.K2_SetActorRotation` _camera_pawn_ref (`KismetMathLibrary.MakeRotator` _returnvalue_roll _returnvalue_pitch (+ _returnvalue_yaw (* AxisValue (`self.RotateSpeed`)))) false))))

(event `InputAction|ZoomOut`
  (params (Key :type "Key Structure"))
  (bind _springarm (`/Game/Main/Blueprints/Player/RTS_CameraPawn_BP.SpringArm` (`self.Camera_Pawn_Ref`)))
  ;[0 1 1] Movement
  ;;[1 1 1] Zoom Out
  (:`Pressed`
    (if (`self.Zoom?`)
      (set `SpringArmComponent.TargetArmLength` (`KismetMathLibrary.FClamp` (+ (`self.ZoomSpeed`) (`SpringArmComponent.TargetArmLength` _springarm)) (`self.MinZoomLim`) (`self.MaxZoomLim`)) _springarm))))

(event `InputAction|Rotate`
  (params (Key :type "Key Structure"))
  (bind _camera_pawn_ref (`self.Camera_Pawn_Ref`))
  (bind (_returnvalue_roll _returnvalue_pitch _returnvalue_yaw) (`KismetMathLibrary.BreakRotator` (`self.K2_GetActorRotation` _camera_pawn_ref)))
  ;[0 1 1] Movement
  ;;[1 1 1] Rotate Y
  (:`Pressed`
    (if (`self.Rotate?`)
      (goto _label_2 :!via `Open`)))
  (:`Released`
    (goto _label_2 :!via `Close`)))

(event `InputAxisKey|MouseY`
  (params (AxisValue :type "Float (single-precision)"))
  (bind _camera_pawn_ref (`self.Camera_Pawn_Ref`))
  (bind (_returnvalue_roll _returnvalue_pitch _returnvalue_yaw) (`KismetMathLibrary.BreakRotator` (`self.K2_GetActorRotation` _camera_pawn_ref)))
  ;[0 1 1] Movement
  ;;[1 1 1] Rotate Y
  (`/Engine/EditorBlueprintResources/StandardMacros.Gate` true :!label _label_2
    (:`Exit`
      (`self.K2_SetActorRotation` _camera_pawn_ref (`KismetMathLibrary.MakeRotator` _returnvalue_roll (`KismetMathLibrary.FClamp` (+ _returnvalue_pitch (* AxisValue (`self.RotateSpeed`))) -20.0 50.0) _returnvalue_yaw) false))))

(event `InputAxis|MoveForward`
  (params (AxisValue :type "Float (single-precision)"))
  (bind _camera_pawn_ref (`self.Camera_Pawn_Ref`))
  (bind _returnvalue (`self.GetTransform` _camera_pawn_ref))
  (bind (_returnvalue_x _returnvalue_y) (`KismetMathLibrary.BreakVector` (+ (`KismetMathLibrary.TransformDirection` _returnvalue (`KismetMathLibrary.MakeVector` (* (* AxisValue (`self.DefaultMovementSpeed`)) (`self.ModifierMovementSpeed`)))) (.location _returnvalue))))
  ;[0 1 1] Movement
  ;;[1 1 1] Camare Move F/B
  (`self.K2_SetActorLocation` _camera_pawn_ref (`KismetMathLibrary.MakeVector` _returnvalue_x _returnvalue_y 110.0) true false))

(event `InputAction|RotateReset`
  (params (Key :type "Key Structure"))
  (bind _camera_pawn_ref (`self.Camera_Pawn_Ref`))
  (bind _returnvalue_roll (`KismetMathLibrary.BreakRotator` (`self.K2_GetActorRotation` _camera_pawn_ref)))
  ;[0 1 1] Movement
  ;;[0 1 0] Resets
  ;;;[1 1 1] Rotate Reset
  (:`Pressed`
    (if (`self.Rotate?`)
      (`self.K2_SetActorRotation` _camera_pawn_ref (`KismetMathLibrary.MakeRotator` _returnvalue_roll) false))))

(event `InputAction|CameraSpeedModifier`
  (params (Key :type "Key Structure"))
  ;[0 1 1] Movement
  ;;[1 1 1] Camera Speed Modifier
  (:`Pressed`
    (set `self.ModifierMovementSpeed` 2.0)
    (set `self.EdgeScrollSpeed` 0.05))
  (:`Released`
    (set `self.ModifierMovementSpeed` 1.0)
    (set `self.EdgeScrollSpeed` 0.025)))

(event `InputAction|ZoomReset`
  (params (Key :type "Key Structure"))
  ;[0 1 1] Movement
  ;;[0 1 0] Resets
  ;;;[1 1 1] Zoom Reset
  (:`Pressed`
    (if (`self.Zoom?`)
      (set `SpringArmComponent.TargetArmLength` 1500.0 (`/Game/Main/Blueprints/Player/RTS_CameraPawn_BP.SpringArm` (`self.Camera_Pawn_Ref`))))))

(event `InputAxis|MoveRight`
  (params (AxisValue :type "Float (single-precision)"))
  (bind _camera_pawn_ref (`self.Camera_Pawn_Ref`))
  (bind _returnvalue (`self.GetTransform` _camera_pawn_ref))
  (bind (_returnvalue_x _returnvalue_y) (`KismetMathLibrary.BreakVector` (+ (`KismetMathLibrary.TransformDirection` _returnvalue (`KismetMathLibrary.MakeVector` 0.0 (* (* AxisValue (`self.DefaultMovementSpeed`)) (`self.ModifierMovementSpeed`)))) (.location _returnvalue))))
  ;[0 1 1] Movement
  ;;[1 1 1] Camera Move R/L
  (`self.K2_SetActorLocation` _camera_pawn_ref (`KismetMathLibrary.MakeVector` _returnvalue_x _returnvalue_y 110.0) true false))

(event `InputAxisKey|MouseX`
  (params (AxisValue :type "Float (single-precision)"))
  ;[0 1 1] Movement
  ;;[1 1 1] Edge Scrolling
  (if (not (`/Game/Main/Blueprints/Widgets/GameTime_WBP.Pause?` (`/Game/Main/Blueprints/Widgets/Main_WBP.GameTime_WBP` (`self.Main_HUD`)))) :!label _label_3
    (bind _newparam (`self.EdgeScrollingFunc`))
    (`self.K2_AddActorLocalOffset` (`self.Camera_Pawn_Ref`) _newparam true false)))

(event `InputAxisKey|MouseY`
  (params (AxisValue :type "Float (single-precision)"))
  ;[0 1 1] Movement
  ;;[1 1 1] Edge Scrolling
  (goto _label_3))

(event `Key|V`
  (params (Key :type "Key Structure"))
  (bind (_relativecoursorlocationingame_x _relativecoursorlocationingame_y) (`KismetMathLibrary.BreakVector` (`/Game/Main/Blueprints/Libraries/RTS_FuncLib_BP.SetCursorWorldPosition` self 10000.0)))
  ;[1 0 0] TEMPORARY
  (:`Pressed`
    (`|SpawnActorFromClass` "/Game/Main/Units/UnitMaster_BP.UnitMaster_BP_C" (`KismetMathLibrary.MakeTransform` (`KismetMathLibrary.MakeVector` _relativecoursorlocationingame_x _relativecoursorlocationingame_y 115.0)) "Undefined" "OverrideRootScale" null null)))

(event `InputAction|SeconderyAction`
  (params (Key :type "Key Structure"))
  (bind (_hitresult _returnvalue) (`self.GetHitResultUnderCursorByChannel` self "TraceTypeQuery1" true))
  ;[0 0 0] Secondary
  (:`Pressed`
    (if (`self.IsInBuildingMode?`)
      (`self.DestroyPreview`)
      (elif (`self.IsSelected?`)
        (if _returnvalue
          (set `self.TargetLocation` (`.Location` (`GameplayStatics.BreakHitResult` _hitresult)))
          (`|ExecutionSequence`
            (:`then_0`
              (bind _previouslocationdecal (`self.PreviousLocationDecal`)
                (:`then`
                  (`ActorComponent.K2_DestroyComponent` _previouslocationdecal)
                  (bind _returnvalue_2 (`AIBlueprintHelperLibrary.GetAIController` (stale _array_element)))
                  (`self.StopMovement` _returnvalue_2))
                (:`else`
                  _))
              (bind _returnvalue_3 (`GameplayStatics.SpawnDecalAtLocation` "/Game/Main/Assets/Materials/Decals/MovementLocationDecal.MovementLocationDecal" (32.0 64.0 64.0) (`self.TargetLocation`)))
              (set `self.PreviousLocationDecal` _returnvalue_3))
            (:`then_1`
              (for _array_element (`self.SelectedUnits`)
                (`self.StopMovement` _returnvalue_2)
                (`AITask_MoveTo.AIMoveTo` _returnvalue_2 (`self.TargetLocation`) null 10.0
                  (:`OnMoveFinished`
                    (bind _previouslocationdecal_2 (`self.PreviousLocationDecal`)
                      (:`then`
                        (`ActorComponent.K2_DestroyComponent` _previouslocationdecal_2))
                      (:`else`))))))))))))

(event `self.ReceiveTick`
  (params (DeltaSeconds :type "Float (single-precision)"))
  ;[0 1 0] EventTick
  (set `self.Delta` DeltaSeconds)
  (`|ExecutionSequence`
    (:`then_0`
      (if (`self.IsHoldingInput?`)
        (`self.UpdateSelection`)))))

(event `UpdateSelection`
  ;[0 0 0] Secondary
  ;;[0 0.2025 0.3469] UnitSelection
  (if (`self.IsHoldingInput?`)
    (set `self.HoldingTime` (+ (`self.HoldingTime`) (`self.Delta`)))
    (message `/Game/Main/Blueprints/Libraries/RTS_MarqueeSelection_IF.OnInputHold` (`self.HUD`))))

(event `InputAction|PrimaryAction`
  (params (Key :type "Key Structure"))
  (bind _preview_ref (`self.Preview_Ref`))
  ;[1 1 1] Primary
  (:`Pressed`
    (if (`self.IsInBuildingMode?`)
      (if (not (`/Game/Main/Blueprints/Buildings/RTS_BuildingMaster_BP.CheckOverlap` _preview_ref))
        (`/Game/Main/Blueprints/Buildings/RTS_BuildingMaster_BP.Place` _preview_ref)
        (bind (_non_busy_nearest_unit_s_aicontroller _unit) (`self.GetNearestUnitToBuilding`))
        (set `self.Builder_Ref` _unit)
        (`self.StopMovement` _non_busy_nearest_unit_s_aicontroller)
        (`AITask_MoveTo.AIMoveTo` _non_busy_nearest_unit_s_aicontroller (0.0 0.0 0.0) (`self.Preview_Ref`) 10.0
          (:`then`
            (`/Game/Main/Blueprints/Buildings/RTS_BuildingMaster_BP.Colide` (`self.Preview_Ref`))
            (`self.SetBuildingModeActive` false)
            (`self.DeselectUnits`))
          (:`OnMoveFinished`
            (`/Game/Main/Blueprints/Buildings/RTS_BuildingMaster_BP.Building` (`self.Preview_Ref`))
            (set `self.Preview_Ref` null)
            (set `/Game/Main/Units/UnitMaster_BP.Busy` true (`self.Builder_Ref`)))))
      (else
        (`self.SelectBuilding`
          (:`Else`
            (`self.StartUnitSelection`)
            (`Widget.SetVisibility` (`/Game/Main/Blueprints/Widgets/Main_WBP.BuildingInfo` (`self.Main_HUD`)) "Hidden"))))))
  (:`Released`
    (if (not (`self.IsInBuildingMode?`))
      (`self.StopSelectingUnits`))
    (`self.-IsAnyWorkerSelected`)))

(fn `-IsAnyWorkerSelected`
  (bind _buildingvariants (`/Game/Main/Blueprints/Widgets/Main_WBP.BuildingVariants` (`self.Main_HUD`)))
  (for _array_element (`self.SelectedUnits`)
    (if (and (not (`/Game/Main/Units/UnitMaster_BP.Busy` _array_element)) (`self.IsSelected?`))
      (`Widget.SetVisibility` _buildingvariants "Visible")
      (else
        (`Widget.SetVisibility` _buildingvariants "Hidden")))))

(fn `DeselectUnits`
  (message `/Game/Main/Blueprints/Libraries/RTS_MarqueeSelection_IF.OnInputStart` (`self.HUD`))
  (set `self.HoldingTime` 0.0))

(fn `DestroyPreview`
  (bind _preview_ref (`self.Preview_Ref`)
    (:`then`
      (`self.K2_DestroyActor` _preview_ref))
    (:`else`
      _))
  (`self.SetBuildingModeActive` false))

(fn `EdgeScrollingFunc`
  (returns (NewParam :type "Vector Structure"))
  (bind _returnvalue_x (`KismetMathLibrary.BreakVector2D` (`WidgetLayoutLibrary.GetViewportSize`)))
  (bind (_returnvalue_x_2 _returnvalue_y) (`KismetMathLibrary.BreakVector2D` (`WidgetLayoutLibrary.GetViewportSize`)))
  (bind (_locationx _locationy) (`self.GetMousePosition`))
  (bind (_returnvalue_x_3 _returnvalue_y_2) (`KismetMathLibrary.BreakVector2D` (`WidgetLayoutLibrary.GetViewportSize`)))
  (bind _returnvalue (/ (`self.GetMousePosition`) _returnvalue_x))
  (bind _returnvalue_2 (/ (`.LocationY` (`self.GetMousePosition`)) _returnvalue_y_2))
  (bind (_returnvalue_x_4 _returnvalue_y_3 _returnvalue_z) (`KismetMathLibrary.BreakVector` (`KismetMathLibrary.MakeVector` (* (* (- (/ _returnvalue_y 2.0) _locationy) (`self.EdgeScrollSpeed`)) (/ _returnvalue_x_2 _returnvalue_y)) (* (- (/ _returnvalue_x_2 2.0) _locationx) (* (`self.EdgeScrollSpeed`) -1.0)))))
  (if (or (or (>= _returnvalue_2 0.985) (<= _returnvalue_2 0.015)) (or (>= _returnvalue 0.985) (<= _returnvalue 0.015)))
    (return (`KismetMathLibrary.MakeVector` _returnvalue_x_4 _returnvalue_y_3 _returnvalue_z))
    (else
      (return (0.0 0.0 0.0)))))

(fn `GetNearestUnitToBuilding`
  (returns (`Non Busy Nearest Unit's AIController` :type "AIController Object Reference") (Unit :type "/Game/Main/Units/UnitMaster_BP Object Reference"))
  (locals (Unit_L :type "/Game/Main/Units/UnitMaster_BP Object Reference") (MinDistance_L :type "Float (double-precision)" :default 10000.0))
  (bind _unit_l (`local.Unit_L`))
  (for _array_element (`self.SelectedUnits`)
    (bind _returnvalue (`KismetMathLibrary.Vector_Distance` (`self.K2_GetActorLocation` _array_element) (`self.K2_GetActorLocation` (`self.Preview_Ref`))))
    (if (and (<= _returnvalue (`local.MinDistance_L`)) (not (`/Game/Main/Units/UnitMaster_BP.Busy` _array_element)))
      (set `local.MinDistance_L` _returnvalue)
      (set `local.Unit_L` _array_element)))
  (return (`AIBlueprintHelperLibrary.GetAIController` _unit_l) _unit_l))

(fn `SetBuildingModeActive`
  (params (IsActive :type Boolean))
  (set `self.IsInBuildingMode?` IsActive)
  (return))

(fn `SetHUDVisibility`
  (params (GaneTimeHUD :type "ESlateVisibility Enum" :default "Visible"))
  (`Widget.SetVisibility` (`self.Main_HUD`) GaneTimeHUD))

(fn `SetSelectedUnits`
  (params (`Selected Units` :type "Array of /Game/Main/Units/UnitMaster_BP Object Reference"))
  (set `self.SelectedUnits` `Selected Units`)
  (if (>= (`KismetArrayLibrary.Array_LastIndex` (`self.SelectedUnits`)) 0)
    (set `self.IsSelected?` true)))

(fn `StartUnitSelection`
  (message `/Game/Main/Blueprints/Libraries/RTS_MarqueeSelection_IF.OnInputStart` (`self.HUD`))
  (set `self.HoldingTime` 0.0)
  (set `self.IsHoldingInput?` true))

(fn `UserConstructionScript`)