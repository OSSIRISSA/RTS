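; SunRotation_BP is a day-cycle actor that rotates the sun in step with the RTS game speed.
; On BeginPlay it reads the speed from RTS_GameState_BP and binds to its game speed counter.
; Each tick, SetGameTime turns delta time, speed and GameTime into a scaled pitch rotation for SunRef.
; It then calls UpdateSunDirection on SkySphereRef so the sky follows the sun.
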(event `self.ReceiveBeginPlay`
  (bind _asrts_game_state_bp (cast `/Game/Main/Blueprints/GameSettings/RTS_GameState_BP` (`GameplayStatics.GetGameState`)))
  (set `self.GameState_Ref` _asrts_game_state_bp)
  (add `/Game/Main/Blueprints/GameSettings/RTS_GameState_BP.GameSpeedCounter` (`self.GameState_Ref`) (`|CreateDelegate` :!event `GetGameSpeed`))
  (bind _gamespeed (`/Game/Main/Blueprints/GameSettings/RTS_GameState_BP.GetGameSpeed` (`self.GameState_Ref`)))
  (set `self.GameSpeed` _gamespeed))

(event `GetGameSpeed`
  (params (GameSpeed :type "Float (double-precision)"))
  (set `self.GameSpeed` GameSpeed))

(event `self.ReceiveTick`
  (params (DeltaSeconds :type "Float (single-precision)"))
  (`self.K2_AddActorLocalRotation` (`self.SunRef`) (`KismetMathLibrary.MakeRotator` 0.0 (* 10 (`/Game/Main/Blueprints/Library/RTS_FuncLib_BP.SetGameTime` DeltaSeconds (`self.GameSpeed`) (`self.GameTime`)))) false false)
  (`/Engine/EngineSky/BP_Sky_Sphere.UpdateSunDirection` (`self.SkySphereRef`)))

(fn `UserConstructionScript`)