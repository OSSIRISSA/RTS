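; TimeSphere is the game clock, tracking the current day and time of day through a looping DayCycle timeline.
; The timeline feeds MovementSec and increments Day each time it finishes, while Tick combines both into the TimeVar timespan.
; UpdateGameSpeed sets the timeline's play rate from TimeSpeed.
; Nodes for sun rotation, light intensity and sky sphere updates exist but are disconnected, so lighting is not driven here.
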(event `self.ReceiveTick`
  (params (DeltaSeconds :type "Float (single-precision)"))
  (`self.Time`))

(event `self.ReceiveBeginPlay`
  (bind (_direction _y_sun_pitch _z_sun_yaw _time _skylight_intensity _dirlight_intensity) (`Timeline|DayCycle` :`NewTime` (`self.Start_Time`) :!via `PlayFromStart` :!label _label)
    (:`Update`
      (set `self.Movement(sec)` _time))
    (:`Finished`
      (`self.Day_Tick`)
      (goto _label :!via `PlayFromStart`))))

(event `UpdateGameSpeed`
  (`TimelineComponent.SetPlayRate` (`self.DayCycle`) (`self.Time_Speed`)))

(fn `Day_Tick`
  (set `self.Day` (+ (`self.Day`) 1)))

(fn `Time`
  (set `self.Time_Var` (`KismetMathLibrary.MakeTimespan` (`self.Day`) 0 0 (`KismetMathLibrary.FTrunc` (`self.Movement(sec)`))))
  (return))

(fn `UserConstructionScript`)