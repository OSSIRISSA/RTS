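; TimeSphere is a day-night cycle Blueprint that drives the sun, sky lighting and game clock from the Day_Cycle timeline.
; Construction sets the play rate from TimeSpeed, BeginPlay seeks to StartTime, and each finish increments Day and restarts the timeline.
; Tick builds a Timespan from day and timeline time, applies timeline values to directional light rotation and both light intensities, then refreshes the sky sphere's sun direction.
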(event `self.ReceiveTick`
  (params (DeltaSeconds :type "Float (single-precision)"))
  (`self.Time`)
  (set `self.Movement(sec)` (stale `self.ReceiveBeginPlay` _time))
  (`self.K2_SetActorRotation` (`self.Dir_Light`) (`KismetMathLibrary.MakeRotator` 0.0 (stale `self.ReceiveBeginPlay` _y_sun_pitch) (stale `self.ReceiveBeginPlay` _z_sun_yaw)) false)
  (`SkyLightComponent.SetIntensity` (`SkyLight.LightComponent` (`self.Sky_Light`)) (stale `self.ReceiveBeginPlay` _skylight_intensity))
  (`LightComponent.SetIntensity` (`Light.LightComponent` (`self.Dir_Light`)) (stale `self.ReceiveBeginPlay` _dirlight_intensity))
  (`/Engine/EngineSky/BP_Sky_Sphere.UpdateSunDirection` (`self.SkySphere_BP`)))

(event `self.ReceiveBeginPlay`
  (bind (_direction _y_sun_pitch _z_sun_yaw _time _skylight_intensity _dirlight_intensity) (`Timeline|Day_Cycle` :`NewTime` (`self.Start_Time`) :!via `SetNewTime` :!label _label)
    (:`Finished`
      (`self.Day_Tick`)
      (goto _label :!via `PlayFromStart`))))

(fn `Day_Tick`
  (set `self.Day` (+ (`self.Day`) 1)))

(fn `Time`
  (set `self.Time_Var` (`KismetMathLibrary.MakeTimespan` (`self.Day`) 0 0 (`KismetMathLibrary.FTrunc` (`self.Movement(sec)`))))
  (return))

(fn `UserConstructionScript`
  (`TimelineComponent.SetPlayRate` (`self.Day_Cycle`) (`self.Time_Speed`)))