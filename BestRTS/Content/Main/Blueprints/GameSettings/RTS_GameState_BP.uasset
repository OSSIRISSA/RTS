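; RTS game state that runs the in-game clock and calendar, seeded from initial time and date values at BeginPlay.
; Each tick, SetGameTime advances GameTime by game speed and yields a day count, which SetClock and SetCalendar convert into time and rolling date, printed on screen.
; Both functions share the GameDate array.
; UpdateGameSpeed writes the scaled default speed into GameTime, not GameSpeed, and passes it to CallGameSpeedCounter.
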(event `self.ReceiveBeginPlay`
  (`|ExecutionSequence`
    (:`then_0`
      (`self.ReferenceCast`))
    (:`then_1`
      (set `self.GameTime` (+ (`KismetMathLibrary.Conv_IntToDouble` (`self.Hours`)) (/ (`KismetMathLibrary.Conv_IntToDouble` (`self.Minutes`)) 60.0) (/ (`KismetMathLibrary.Conv_IntToDouble` (`self.Hours`)) 3600.0)))
      (set `self.GameDate` (`|MakeArray` (`self.Day`) (`self.Month`) (`self.Year`))))
    (:`then_2`
      (set `self.GameSpeed` (`self.DefaultGameSpeed`)))))

(event `self.ReceiveTick`
  (params (DeltaSeconds :type "Float (single-precision)"))
  (bind (_gametime _day) (`/Game/Main/Blueprints/Library/RTS_FuncLib_BP.SetGameTime` DeltaSeconds (`self.GameSpeed`) (`self.GameTime`)))
  (set `self.GameTime` _gametime)
  (set `self.DayCounter` _day)
  (`self.SetClock`)
  (`self.SetCalendar`))

(event `/Game/Main/Blueprints/Library/RTS_GameTime_IF.UpdateGameSpeed`
  (params (SpeedMultyplier :type "Float (single-precision)"))
  (bind _output_get (set `self.SpeedMultiplier` SpeedMultyplier))
  (bind _output_get_2 (set `self.GameTime` (* _output_get (`self.DefaultGameSpeed`))))
  (`self.GameSpeedCounter` _output_get_2))

(fn `SetCalendar`
  (bind _output_get (set `self.Day` (+ (`self.DayCounter`) (`self.Day`))))
  (if (> _output_get (`KismetMathLibrary.DaysInMonth` (`self.Year`) (`self.Month`)))
    (set `self.Day` 1)
    (set `self.Month` (+ (`self.Month`) 1)))
  (if (> (`self.Month`) 12)
    (set `self.Month` 1)
    (set `self.Year` (+ (`self.Year`) 1)))
  (bind _output_get_2 (set `self.GameDate` (`|MakeArray` (`self.Day`) (`self.Month`) (`self.Year`))))
  (`KismetSystemLibrary.PrintString` (`KismetStringLibrary.BuildString_Int` (`KismetStringLibrary.BuildString_Int` (`KismetStringLibrary.Conv_IntToString` (`|GetArrayItem` _output_get_2)) "/" (`|GetArrayItem` _output_get_2 1)) "/" (`|GetArrayItem` _output_get_2 2)) true true (struct :`G` 0.66 :`B` 1.0 :`A` 1.0) 0.0))

(fn `SetClock`
  (bind (_remainder _returnvalue) (`KismetMathLibrary.FMod` (* (`self.GameTime`) 3600.0) 60.0))
  (bind (_remainder_2 _returnvalue_2) (`KismetMathLibrary.FMod` (`KismetMathLibrary.Conv_IntToDouble` _returnvalue) 60.0))
  (set `self.Seconds` (`KismetMathLibrary.FFloor` _remainder))
  (set `self.Minutes` (`KismetMathLibrary.FFloor` _remainder_2))
  (set `self.Hours` (`KismetMathLibrary.FFloor` (`KismetMathLibrary.FMod` (`KismetMathLibrary.Conv_IntToDouble` _returnvalue_2) 24.0)))
  (bind _output_get (set `self.GameDate` (`|MakeArray` (`self.Seconds`) (`self.Minutes`) (`self.Hours`))))
  (`KismetSystemLibrary.PrintString` (`KismetStringLibrary.BuildString_Int` (`KismetStringLibrary.BuildString_Int` (`KismetStringLibrary.Conv_IntToString` (`|GetArrayItem` _output_get 2)) ":" (`|GetArrayItem` _output_get 1)) ":" (`|GetArrayItem` _output_get)) true true (struct :`G` 0.66 :`B` 1.0 :`A` 1.0) 0.0)
  (return))

(fn `UserConstructionScript`)