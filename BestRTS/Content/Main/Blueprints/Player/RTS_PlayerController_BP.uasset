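; RTS player controller that drives the camera pawn and shows the game-time HUD widget.
; BeginPlay caches the camera pawn and TimeSphere references, then creates the widget.
; Input zooms via clamped spring-arm length, rotates through gated mouse axes with clamped pitch, and pans at a fixed height with a speed modifier.
; Mouse movement also triggers swept edge scrolling, offsetting the pawn by cursor distance from screen center when near viewport borders.
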(event `self.ReceiveBeginPlay`
  ;[1 0 0] BeginPlay
  (`|ExecutionSequence`
    (:`then_0`
      (`self.ReferenceCast`))
    (:`then_1`
      (`self.SpawnWidgets`)
      (`UserWidget.AddToViewport` (`self.GameTime_WB_Ref`) 0)
      (`self.SetHUDVisibility` "Visible"))))

(event `InputAction|ZoomIn`
  (params (Key :type "Key Structure"))
  (bind _springarm (`/Game/Main/Blueprints/Player/RTS_CameraPawn_BP.SpringArm` (`self.Camera_Pawn_Ref`)))
  ;[0 1 1] Movement
  ;;[1 1 1] Zoom In
  (:`Pressed`
    (if (`self.Zoom?`)
      (set `SpringArmComponent.TargetArmLength` (`KismetMathLibrary.FClamp` (- (`SpringArmComponent.TargetArmLength` _springarm) (`self.ZoomSpeed`)) (`self.MinZoomLim`) (`self.MaxZoomLim`)) _springarm))))

(event `InputAction|Rotate`
  (params (Key :type "Key Structure"))
  (bind _camera_pawn_ref (`self.Camera_Pawn_Ref`))
  (bind (_returnvalue_roll _returnvalue_pitch _returnvalue_yaw) (`KismetMathLibrary.BreakRotator` (`self.K2_GetActorRotation` _camera_pawn_ref)))
  ;[0 1 1] Movement
  ;;[1 1 1] Rotate X
  (:`Pressed`
    (if (`self.Rotate?`)
      (goto _label :!via `Open`)))
  (:`Released`
    (goto _label :!via `Close`)))

(event `InputAxisKey|MouseX`
  (params (AxisValue :type "Float (single-precision)"))
  (bind _camera_pawn_ref (`self.Camera_Pawn_Ref`))
  (bind (_returnvalue_roll _returnvalue_pitch _returnvalue_yaw) (`KismetMathLibrary.BreakRotator` (`self.K2_GetActorRotation` _camera_pawn_ref)))
  ;[0 1 1] Movement
  ;;[1 1 1] Rotate X
  (`/Engine/EditorBlueprintResources/StandardMacros.Gate` true :!label _label
    (:`Exit`
      (`self.K2_SetActorRotation` _camera_pawn_ref (`KismetMathLibrary.MakeRotator` _returnvalue_roll _returnvalue_pitch (+ _returnvalue_yaw (* AxisValue (`self.RotateSpeed`)))) false))))

(event `InputAction|ZoomOut`
  (params (Key :type "Key Structure"))
  (bind _springarm (`/Game/Main/Blueprints/Player/RTS_CameraPawn_BP.SpringArm` (`self.Camera_Pawn_Ref`)))
  ;[0 1 1] Movement
  ;;[1 1 1] Zoom Out
  (:`Pressed`
    (if (`self.Zoom?`)
      (set `SpringArmComponent.TargetArmLength` (`KismetMathLibrary.FClamp` (+ (`self.ZoomSpeed`) (`SpringArmComponent.TargetArmLength` _springarm)) (`self.MinZoomLim`) (`self.MaxZoomLim`)) _springarm))))

(event `InputAction|Rotate`
  (params (Key :type "Key Structure"))
  (bind _camera_pawn_ref (`self.Camera_Pawn_Ref`))
  (bind (_returnvalue_roll _returnvalue_pitch _returnvalue_yaw) (`KismetMathLibrary.BreakRotator` (`self.K2_GetActorRotation` _camera_pawn_ref)))
  ;[0 1 1] Movement
  ;;[1 1 1] Rotate Y
  (:`Pressed`
    (if (`self.Rotate?`)
      (goto _label_2 :!via `Open`)))
  (:`Released`
    (goto _label_2 :!via `Close`)))

(event `InputAxisKey|MouseY`
  (params (AxisValue :type "Float (single-precision)"))
  (bind _camera_pawn_ref (`self.Camera_Pawn_Ref`))
  (bind (_returnvalue_roll _returnvalue_pitch _returnvalue_yaw) (`KismetMathLibrary.BreakRotator` (`self.K2_GetActorRotation` _camera_pawn_ref)))
  ;[0 1 1] Movement
  ;;[1 1 1] Rotate Y
  (`/Engine/EditorBlueprintResources/StandardMacros.Gate` true :!label _label_2
    (:`Exit`
      (`self.K2_SetActorRotation` _camera_pawn_ref (`KismetMathLibrary.MakeRotator` _returnvalue_roll (`KismetMathLibrary.FClamp` (+ _returnvalue_pitch (* AxisValue (`self.RotateSpeed`))) -20.0 50.0) _returnvalue_yaw) false))))

(event `InputAxis|MoveForward`
  (params (AxisValue :type "Float (single-precision)"))
  (bind _camera_pawn_ref (`self.Camera_Pawn_Ref`))
  (bind _returnvalue (`self.GetTransform` _camera_pawn_ref))
  (bind (_returnvalue_x _returnvalue_y) (`KismetMathLibrary.BreakVector` (+ (`KismetMathLibrary.TransformDirection` _returnvalue (`KismetMathLibrary.MakeVector` (* (* AxisValue (`self.DefaultMovementSpeed`)) (`self.ModifierMovementSpeed`)))) (.location _returnvalue))))
  ;[0 1 1] Movement
  ;;[1 1 1] Camare Move F/B
  (`self.K2_SetActorLocation` _camera_pawn_ref (`KismetMathLibrary.MakeVector` _returnvalue_x _returnvalue_y 200.0) true false))

(event `InputAction|RotateReset`
  (params (Key :type "Key Structure"))
  (bind _camera_pawn_ref (`self.Camera_Pawn_Ref`))
  (bind _returnvalue_roll (`KismetMathLibrary.BreakRotator` (`self.K2_GetActorRotation` _camera_pawn_ref)))
  ;[0 1 1] Movement
  ;;[0 1 0] Resets
  ;;;[1 1 1] Rotate Reset
  (:`Pressed`
    (if (`self.Rotate?`)
      (`self.K2_SetActorRotation` _camera_pawn_ref (`KismetMathLibrary.MakeRotator` _returnvalue_roll) false))))

(event `InputAction|CameraSpeedModifier`
  (params (Key :type "Key Structure"))
  ;[0 1 1] Movement
  ;;[1 1 1] Camera Speed Modifier
  (:`Pressed`
    (set `self.ModifierMovementSpeed` 2.0))
  (:`Released`
    (set `self.ModifierMovementSpeed` 1.0)))

(event `InputAction|ZoomReset`
  (params (Key :type "Key Structure"))
  ;[0 1 1] Movement
  ;;[0 1 0] Resets
  ;;;[1 1 1] Zoom Reset
  (:`Pressed`
    (if (`self.Zoom?`)
      (set `SpringArmComponent.TargetArmLength` 1500.0 (`/Game/Main/Blueprints/Player/RTS_CameraPawn_BP.SpringArm` (`self.Camera_Pawn_Ref`))))))

(event `InputAxis|MoveRight`
  (params (AxisValue :type "Float (single-precision)"))
  (bind _camera_pawn_ref (`self.Camera_Pawn_Ref`))
  (bind _returnvalue (`self.GetTransform` _camera_pawn_ref))
  (bind (_returnvalue_x _returnvalue_y) (`KismetMathLibrary.BreakVector` (+ (`KismetMathLibrary.TransformDirection` _returnvalue (`KismetMathLibrary.MakeVector` 0.0 (* (* AxisValue (`self.DefaultMovementSpeed`)) (`self.ModifierMovementSpeed`)))) (.location _returnvalue))))
  ;[0 1 1] Movement
  ;;[1 1 1] Camera Move R/L
  (`self.K2_SetActorLocation` _camera_pawn_ref (`KismetMathLibrary.MakeVector` _returnvalue_x _returnvalue_y 200.0) true false))

(event `InputAxisKey|MouseX`
  (params (AxisValue :type "Float (single-precision)"))
  ;[0 1 1] Movement
  ;;[1 1 1] Edge Scrolling
  (bind _newparam (`self.EdgeScrollingFunc` :!label _label_3))
  (`self.K2_AddActorLocalOffset` (`self.Camera_Pawn_Ref`) _newparam true false))

(event `InputAxisKey|MouseY`
  (params (AxisValue :type "Float (single-precision)"))
  ;[0 1 1] Movement
  ;;[1 1 1] Edge Scrolling
  (goto _label_3))

(event `self.ReceiveTick`
  (params (DeltaSeconds :type "Float (single-precision)")))

(fn `EdgeScrollingFunc`
  (returns (NewParam :type "Vector Structure"))
  (bind _returnvalue_x (`KismetMathLibrary.BreakVector2D` (`WidgetLayoutLibrary.GetViewportSize`)))
  (bind (_returnvalue_x_2 _returnvalue_y) (`KismetMathLibrary.BreakVector2D` (`WidgetLayoutLibrary.GetViewportSize`)))
  (bind (_locationx _locationy) (`self.GetMousePosition`))
  (bind (_returnvalue_x_3 _returnvalue_y_2) (`KismetMathLibrary.BreakVector2D` (`WidgetLayoutLibrary.GetViewportSize`)))
  (bind _returnvalue (/ (`self.GetMousePosition`) _returnvalue_x))
  (bind _returnvalue_2 (/ (`.LocationY` (`self.GetMousePosition`)) _returnvalue_y_2))
  (if (or (or (>= _returnvalue_2 0.985) (<= _returnvalue_2 0.015)) (or (>= _returnvalue 0.985) (<= _returnvalue 0.015)))
    (return (`KismetMathLibrary.MakeVector` (* (* (- (/ _returnvalue_y 2.0) _locationy) (`self.EdgeScrollSpeed`)) (/ _returnvalue_x_2 _returnvalue_y)) (* (- (/ _returnvalue_x_2 2.0) _locationx) (* (`self.EdgeScrollSpeed`) -1.0))))
    (else
      (return (0.0 0.0 0.0)))))

(fn `SetHUDVisibility`
  (params (GaneTimeHUD :type "ESlateVisibility Enum" :default "Visible"))
  (`Widget.SetVisibility` (`self.GameTime_WB_Ref`) GaneTimeHUD))

(fn `UserConstructionScript`)